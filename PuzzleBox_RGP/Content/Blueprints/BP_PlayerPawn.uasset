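; BP_PlayerPawn is the player's pawn for clicking away non-required BP_Cube blocks.
; On BeginPlay it caches BP_GameMode and the level's BP_BoundingActor, which it stores as its Camera.
; Left click traces from the mouse cursor with persistent debug drawing, notifies the game mode and destroys the hit cube unless it is required.
; The move-object input targets the camera's spring arm rotation but currently adds zero rotation.
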(event Input|EnhancedActionEvents|EnhancedInputActionIA_LeftClick
  (params (ActionValue :type Boolean) (ElapsedSeconds :type Float%20%28double-precision%29) (TriggeredSeconds :type Float%20%28double-precision%29) (InputAction :type Input%20Action%20Object%20Reference :default "/Game/Blueprints/IA_LeftClick.IA_LeftClick"))
  (bind _returnvalue (Game|GetPlayerController 0))
  (bind (_worldlocation _worlddirection) (Game|Player|ConvertMouseLocationToWorldSpace _returnvalue))
  (:Started
    (bind _outhit (Collision|LineTraceByChannel _worldlocation (+ _worldlocation (* _worlddirection 2e+03)) "TraceTypeQuery1" false 0 "Persistent"))
    (if (== (Utilities|GetClass (.HitActor (Collision|BreakHitResult _outhit))) "/Game/Blueprints/BP_Cube.BP_Cube_C")
      (bind _asbp_cube (Utilities|Casting|CastToBP_Cube (.HitActor (Collision|BreakHitResult _outhit))))
      (if (not (Variables|/Game/Blueprints/BP_Cube.BP_Cube_C|GetisRequiredBlock? _asbp_cube))
        (Default|CallOnBlockDestroyed (Variables|Default|GetGameMode) _asbp_cube)
        (Actor|DestroyActor (.HitActor (Collision|BreakHitResult _outhit)))))))

(event Input|EnhancedActionEvents|EnhancedInputActionIA_MoveObject
  (params (ActionValue :type Boolean) (ElapsedSeconds :type Float%20%28double-precision%29) (TriggeredSeconds :type Float%20%28double-precision%29) (InputAction :type Input%20Action%20Object%20Reference :default "/Game/Blueprints/IA_MoveObject.IA_MoveObject"))
  (:Triggered
    (Transformation|AddRelativeRotation (Variables|/Game/Blueprints/BP_BoundingActor.BP_BoundingActor_C|GetSpringArm (Variables|Default|GetCamera)) "0, 0, 0" false false)))

(event EventBeginPlay
  (bind _asbp_game_mode (Utilities|Casting|CastToBP_GameMode (Game|GetGameMode)))
  (Variables|Default|SetGameMode _asbp_game_mode)
  (bind _returnvalue (Actor|GetActorOfClass "/Game/Blueprints/BP_BoundingActor.BP_BoundingActor_C"))
  (bind _asbp_bounding_actor (Utilities|Casting|CastToBP_BoundingActor _returnvalue))
  (Variables|Default|SetCamera _asbp_bounding_actor))

(fn ConstructionScript)