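; BP_GameMode is a game mode that detects when every non-required cube in the level has been destroyed.
; On BeginPlay it sorts all BP_Cube actors by IsRequiredBlock into required and to-destroy lists, then binds BlockDestroyed to the OnBlockDestroyed event.
; Each destroyed block leaves the to-destroy list, and once that list is empty, OnGameFinished is called on every required block.
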(event Custom|BlockDestroyed
  (params (Block :type BP%20Cube%20Object%20Reference))
  (bind _blockstodestroy (Variables|Default|GetBlocksToDestroy))
  (Utilities|Array|RemoveItem _blockstodestroy Block)
  (if (Utilities|Array|IsEmpty _blockstodestroy)
    (for _array_element (Variables|Default|GetRequiredBlocks)
      (Default|CallOnGameFinished _array_element))))

(event EventBeginPlay
  (bind _outactors (Actor|GetAllActorsOfClass "/Game/Blueprints/BP_Cube.BP_Cube_C"))
  (for _array_element _outactors
    (if (Variables|/Game/Blueprints/BP_Cube.BP_Cube_C|GetisRequiredBlock? _array_element)
      (Utilities|Array|Add (Variables|Default|GetRequiredBlocks) _array_element)
      (else
        (Utilities|Array|Add (Variables|Default|GetBlocksToDestroy) _array_element))))
  (EventDispatchers|BindEventtoOnBlockDestroyed (delegate Custom|BlockDestroyed)))

(fn ConstructionScript)