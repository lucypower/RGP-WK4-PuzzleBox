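; Player pawn for a block-removal game built around a single BP_BoundingActor that holds the puzzle's orientation.
; Left click traces under the cursor and destroys any BP_Cube not flagged as required, notifying BP_GameMode first.
; Holding right mouse with Left Shift, which hides the cursor, lets IA_MoveObject rotate the bounding actor around the numpad-selected axis.
; Space bar resets that actor's rotation.
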(event Input|EnhancedActionEvents|EnhancedInputActionIA_LeftClick
  (params (ActionValue :type Boolean) (ElapsedSeconds :type Float%20%28double-precision%29) (TriggeredSeconds :type Float%20%28double-precision%29) (InputAction :type Input%20Action%20Object%20Reference :default "/Game/Blueprints/IA_LeftClick.IA_LeftClick"))
  (bind _returnvalue (Game|GetPlayerController 0))
  (bind (_worldlocation _worlddirection) (Game|Player|ConvertMouseLocationToWorldSpace _returnvalue))
  (:Started
    (bind _outhit (Collision|LineTraceByChannel _worldlocation (+ _worldlocation (* _worlddirection 1e+04)) "TraceTypeQuery1" false 0 "None"))
    (if (== (Utilities|GetClass (.HitActor (Collision|BreakHitResult _outhit))) "/Game/Blueprints/BP_Cube.BP_Cube_C")
      (bind _asbp_cube (Utilities|Casting|CastToBP_Cube (.HitActor (Collision|BreakHitResult _outhit))))
      (if (not (Variables|/Game/Blueprints/BP_Cube.BP_Cube_C|GetisRequiredBlock? _asbp_cube))
        (Default|CallOnBlockDestroyed (Variables|Default|GetGameMode) _asbp_cube)
        (Actor|DestroyActor (.HitActor (Collision|BreakHitResult _outhit)))))))

(event Input|EnhancedActionEvents|EnhancedInputActionIA_MoveObject
  (params (ActionValue :type Float%20%28double-precision%29) (ElapsedSeconds :type Float%20%28double-precision%29) (TriggeredSeconds :type Float%20%28double-precision%29) (InputAction :type Input%20Action%20Object%20Reference :default "/Game/Blueprints/IA_MoveObject.IA_MoveObject"))
  (bind _cubes (Variables|Default|GetCubes))
  (bind _rootcomponent (Variables|/Script/Engine.Actor|GetRootComponent _cubes))
  (if (Variables|Default|GetcanRotate?)
    (if (not (Variables|/Script/Engine.PlayerController|GetbShowMouseCursor (Game|GetPlayerController 0)))
      (switch string (Variables|Default|Getaxis)
        (:x
          (Transformation|AddRelativeRotation _rootcomponent (Math|Rotator|MakeRotator ActionValue 0.0 0.0) false false))
        (:y
          (Transformation|AddRelativeRotation _rootcomponent (Math|Rotator|MakeRotator 0.0 ActionValue 0.0) false false))
        (:z
          (Transformation|AddRelativeRotation _rootcomponent (Math|Rotator|MakeRotator 0.0 0.0 ActionValue) false false))))))

(event EventBeginPlay
  (bind _asbp_game_mode (Utilities|Casting|CastToBP_GameMode (Game|GetGameMode)))
  (Variables|Default|SetGameMode _asbp_game_mode)
  (bind _returnvalue (Actor|GetActorOfClass "/Game/Blueprints/BP_BoundingActor.BP_BoundingActor_C"))
  (Variables|Default|SetCubes _returnvalue))

(event Input|MouseEvents|RightMouseButton
  (params (Key :type Key%20Structure :default "None"))
  (:Pressed
    (Variables|Default|SetcanRotate? true))
  (:Released
    (Variables|Default|SetcanRotate? false)))

(event Input|KeyboardEvents|SpaceBar
  (params (Key :type Key%20Structure :default "None"))
  (:Pressed
    (Transformation|SetRelativeRotation (Variables|/Script/Engine.Actor|GetRootComponent (Variables|Default|GetCubes)) "0, 0, 0" false false)))

(event Input|KeyboardEvents|LeftShift
  (params (Key :type Key%20Structure :default "None"))
  (bind _returnvalue (Game|GetPlayerController 0))
  (:Pressed
    (Variables|/Script/Engine.PlayerController|SetbShowMouseCursor _returnvalue false))
  (:Released
    (Variables|/Script/Engine.PlayerController|SetbShowMouseCursor _returnvalue true)))

(event Input|KeyboardEvents|NumPadOne
  (params (Key :type Key%20Structure :default "None"))
  (:Pressed
    (Variables|Default|Setaxis "x")))

(event Input|KeyboardEvents|NumPadTwo
  (params (Key :type Key%20Structure :default "None"))
  (:Pressed
    (Variables|Default|Setaxis "y")))

(event Input|KeyboardEvents|NumPadThree
  (params (Key :type Key%20Structure :default "None"))
  (:Pressed
    (Variables|Default|Setaxis "z")))

(fn ConstructionScript)