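; BP_Cube is a cube actor that shows a configurable text label on each of its six faces until the game finishes.
; The construction script and BeginPlay both set the face texts from per-face value variables.
; BeginPlay also binds SetColourMaterial to the OnGameFinished dispatcher, which applies the stored material to the cube and destroys all six text components.
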(event Custom|SetColourMaterial
  (Rendering|Material|SetMaterial (Variables|Default|GetCube) 0 (Variables|Default|GetMaterial))
  (Components|DestroyComponent (Variables|Default|GetTop))
  (Components|DestroyComponent (Variables|Default|GetFront))
  (Components|DestroyComponent (Variables|Default|GetBack))
  (Components|DestroyComponent (Variables|Default|GetRight))
  (Components|DestroyComponent (Variables|Default|GetLeft))
  (Components|DestroyComponent (Variables|Default|GetBottom)))

(event EventBeginPlay
  (Rendering|Components|TextRender|SetText (Variables|Default|GetTop) (Variables|Default|GettopValue))
  (Rendering|Components|TextRender|SetText (Variables|Default|GetBottom) (Variables|Default|GetbottomValue))
  (Rendering|Components|TextRender|SetText (Variables|Default|GetLeft) (Variables|Default|GetleftValue))
  (Rendering|Components|TextRender|SetText (Variables|Default|GetRight) (Variables|Default|GetrightValue))
  (Rendering|Components|TextRender|SetText (Variables|Default|GetFront) (Variables|Default|GetfrontValue))
  (Rendering|Components|TextRender|SetText (Variables|Default|GetBack) (Variables|Default|GetbackValue))
  (EventDispatchers|BindEventtoOnGameFinished (delegate Custom|SetColourMaterial)))

(fn ConstructionScript
  (Rendering|Components|TextRender|SetText (Variables|Default|GetTop) (Variables|Default|GettopValue))
  (Rendering|Components|TextRender|SetText (Variables|Default|GetBottom) (Variables|Default|GetbottomValue))
  (Rendering|Components|TextRender|SetText (Variables|Default|GetLeft) (Variables|Default|GetleftValue))
  (Rendering|Components|TextRender|SetText (Variables|Default|GetRight) (Variables|Default|GetrightValue))
  (Rendering|Components|TextRender|SetText (Variables|Default|GetFront) (Variables|Default|GetfrontValue))
  (Rendering|Components|TextRender|SetText (Variables|Default|GetBack) (Variables|Default|GetbackValue)))